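; BP_WaveSpawner is an enemy wave spawner that spawns its first batch at its own transform on BeginPlay.
; SpawnEnemy loops SpawnedEnemy times, spawning the Enemies class, then adds EnemiesAlive to that count; AddEnemies is incremented and reset without being used.
; EnemiesRemaining binds a respawn event and prints a wave message when none are alive, but nothing here calls it and its SpawnEnemy call is disconnected.
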(event Custom|Init
  (CallFunction|SpawnEnemy))

(event Custom|SpawnEnemy
  (for _index (range 1 (Variables|Default|GetSpawnedEnemy))
    (Game|SpawnActorfromClass (Variables|Default|GetEnemies) (Transformation|GetActorTransform) "AdjustIfPossibleButAlwaysSpawn" "MultiplyWithRoot" 0 0))
  (Math|Integer|IncrementInt (Variables|Default|GetAddEnemies)
    (:%20%20
      (Variables|Default|SetSpawnedEnemy (+ (Variables|Default|GetSpawnedEnemy) (Variables|Default|GetEnemiesAlive)))
      (Variables|Default|SetAddEnemies 0))))

(event EventBeginPlay
  (CallFunction|Init))

(fn ConstructionScript)

(fn EnemiesRemaining
  (if (== (Variables|Default|GetEnemiesAlive) 0)
    (EventDispatchers|BindEventtoRespawnEnemy (EventDispatchers|CreateEvent :!event Custom|SpawnEnemy))
    (Development|PrintString "WaveBegun")))