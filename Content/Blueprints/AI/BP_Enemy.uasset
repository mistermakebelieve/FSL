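; BP_Enemy is an AI enemy character with melee sword and big slam attacks, stat-based health and a health bar widget.
; A looping timer sphere-traces from sword hilt to tip to damage pawns, throttled by DoOnce, while the slam uses a single radius trace at a point.
; Incoming damage lowers a stat in BPCStats.
; Death ragdolls the mesh, requests a WaveSpawner respawn in wave mode, and despawns on a timer.
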(event Custom|Despawn
  ;[0.004712 0.07292 0] Despawn
  (Utilities|Time|SetTimerbyEvent (delegate Custom|DestroySelf) (Variables|Default|GetDespawnTime)))

(event Custom|DamageTrace
  ;[0.004712 0.07292 0] Sword Traces
  (if (not (Variables|Default|GetIsDead?))
    (bind (_outhit _returnvalue) (Collision|SphereTraceForObjects (Transformation|GetWorldLocation (Variables|Default|GetStart%20Sword%20Trace%20Pos)) (Transformation|GetWorldLocation (Variables|Default|GetEnd%20Sword%20Trace%20Pos)) 25.0 (Utilities|Array|MakeArray "ObjectTypeQuery3") false 0 "ForOneFrame"))
    (if _returnvalue
      (Utilities|FlowControl|DoOnce false :!label _label
        (:Completed
          (Game|Damage|ApplyDamage (.HitActor (Collision|BreakHitResult _outhit)) (Variables|Default|GetSwordDamage) 0 0)
          ;[0.6198 0.01517 0] !!!!!This should be based on animation. Get BPI_Enemy, attack function, and use animation delay?
          (Utilities|FlowControl|Delay 0.3)
          (goto _label Reset))))))

(event Custom|DestroySelf
  ;[0.004712 0.07292 0] Despawn
  (Actor|DestroyActor))

(event EventBeginPlay
  (CallFunction|Init))

(event Game|Damage|EventAnyDamage
  (params (Damage :type Float%20%28single-precision%29) (DamageType :type Damage%20Type%20Object%20Reference) (InstigatedBy :type Controller%20Object%20Reference) (DamageCauser :type Actor%20Object%20Reference))
  ;[0.004712 0.07292 0] Damaged
  (Default|AlterStatValue (Variables|Default|GetBPC_Stats) "NewEnumerator0" (* Damage -1.0)))

(event EventDie
  ;[0.004712 0.07292 0] Death
  (Pawn|Components|CharacterMovement|DisableMovement (Variables|Character|GetCharacterMovement))
  (Physics|SetSimulatePhysics (Variables|Character|GetMesh) true)
  (if (Variables|WaveMode|GetWaveMode?)
    (Default|RespawnEnemy (Variables|WaveMode|GetWaveSpawner))
    (CallFunction|Despawn)
    (else
      (CallFunction|Despawn))))

(event EventBeginSwordTrace
  ;[0.004712 0.07292 0] Sword Traces
  (bind _returnvalue (Utilities|Time|SetTimerbyEvent (delegate Custom|DamageTrace) 0.01 true)))

(event EventEndSwordTrace
  ;[0.004712 0.07292 0] Sword Traces
  (if (Utilities|Time|IsValidTimerHandle (stale EventBeginSwordTrace _returnvalue))
    (Utilities|Time|ClearandInvalidateTimerbyHandle (stale EventBeginSwordTrace _returnvalue))))

(event EventPointDamageTrace
  (bind _pointtraceposition (Variables|Default|GetPointTracePosition))
  (bind _returnvalue (Transformation|GetWorldLocation _pointtraceposition))
  ;[0.004712 0.07292 0] Boss slam - this is a sphere hit. Otherwise, get the rotation from the point trace position, pull world rotation and then forward vector then multiply that by a float for End point.
  (bind (_outhit _returnvalue_2) (Collision|SphereTraceForObjects _returnvalue _returnvalue (Variables|Default|GetPointAttackRadius) (Utilities|Array|MakeArray "ObjectTypeQuery3") false 0 "None" true "(R=1.000000,G=0.000000,B=0.000000,A=1.000000)" "(R=0.000000,G=1.000000,B=0.000000,A=1.000000)" 3.0))
  (if _returnvalue_2
    (Game|Damage|ApplyDamage (.HitActor (Collision|BreakHitResult _outhit)) (Variables|Default|GetBigHitDamage) 0 0)))

(fn ConstructionScript)

(fn Init
  (bind _aswb_enemy_health (Utilities|Casting|CastToWB_EnemyHealth (UserInterface|GetWidget (Variables|Default|GetWidget))))
  (Variables|/Game/Blueprints/BPC_Stats.BPC_Stats_C|SetHealth%20Progress%20Bar (Variables|Default|GetBPC_Stats) (Variables|/Game/UI/WB_EnemyHealth.WB_EnemyHealth_C|GetHealthBar _aswb_enemy_health)))

(fn BigAttack
  (bind _returnvalue (Animation|PlayAnimMontage "/Game/Characters/Souls/Combat/BigAttack_Montage.BigAttack_Montage" 1.0 "None"))
  (return _returnvalue))

(fn SwordAttack
  (bind _returnvalue (Animation|PlayAnimMontage "/Game/Characters/Souls/Combat/SwordAttackCombo_Montage.SwordAttackCombo_Montage" 1.0 "None"))
  (return _returnvalue))