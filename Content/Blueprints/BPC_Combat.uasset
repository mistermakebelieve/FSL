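; Player combat component for BP_ThirdPersonCharacter, handling target lock, sword combo attacks and directional dodging.
; Lock-on sphere-traces for a pawn, attaches a marker actor, switches to controller-facing movement and steers control rotation each tick.
; Montage notifies continue or stop the combo based on buffered input, while timer-looped hilt-to-tip traces apply damage, throttled by a fixed delay.
; Dodge montages follow the pressed WASD key when controller-facing, otherwise forward.
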(event Custom|BeginDamageTrace
  ;[0.004712 0.07292 0] Sword Traces
  (bind _returnvalue (Utilities|Time|SetTimerbyEvent (delegate Custom|DamageTrace) 0.01 true)))

(event Custom|DamageTrace
  (bind _playerbp (Variables|Default|GetPlayerBP))
  ;[0.004712 0.07292 0] Sword Traces
  (bind (_outhit _returnvalue) (Collision|SphereTraceForObjects (Transformation|GetWorldLocation (Variables|/Game/ThirdPerson/Blueprints/BP_ThirdPersonCharacter.BP_ThirdPersonCharacter_C|GetStart%20Sword%20Trace%20Pos _playerbp)) (Transformation|GetWorldLocation (Variables|/Game/ThirdPerson/Blueprints/BP_ThirdPersonCharacter.BP_ThirdPersonCharacter_C|GetEnd%20Sword%20Trace%20Pos _playerbp)) 25.0 (Utilities|Array|MakeArray "ObjectTypeQuery3") false 0 "ForOneFrame"))
  (if _returnvalue
    (Utilities|FlowControl|DoOnce false :!label _label
      (:Completed
        (Game|Damage|ApplyDamage (.HitActor (Collision|BreakHitResult _outhit)) (Variables|Default|GetSwordDamage) 0 0)
        ;[0.6198 0.01517 0] !!!!!This is bad. It should be based on animation!!!!!
        (Utilities|FlowControl|Delay 0.3)
        (goto _label Reset)))))

(event Custom|End%20Damage%20Trace
  ;[0.004712 0.07292 0] Sword Traces
  (if (Utilities|Time|IsValidTimerHandle (stale Custom|BeginDamageTrace _returnvalue))
    (Utilities|Time|ClearandInvalidateTimerbyHandle (stale Custom|BeginDamageTrace _returnvalue))))

(event Input|EnhancedActionEvents|EnhancedInputActionIA_Lock
  (params (ActionValue :type Boolean) (ElapsedSeconds :type Float%20%28double-precision%29) (TriggeredSeconds :type Float%20%28double-precision%29) (InputAction :type Input%20Action%20Object%20Reference :default "/Game/ThirdPerson/Input/Actions/IA_Lock.IA_Lock"))
  (bind _returnvalue (Game|GetPlayerCameraManager 0))
  (bind _playerbp (Variables|Default|GetPlayerBP))
  (bind _playerbp_2 (Variables|Default|GetPlayerBP))
  (bind _transformcomponent (Variables|/Script/Engine.PlayerCameraManager|GetTransformComponent _returnvalue))
  (bind _charactermovement (Variables|/Script/Engine.Character|GetCharacterMovement _playerbp_2))
  (bind _charactermovement_2 (Variables|/Script/Engine.Character|GetCharacterMovement _playerbp))
  (bind _returnvalue_2 (Transformation|GetWorldLocation _transformcomponent))
  ;[0 0.06426 0.07292] Target Lock
  (:Started
    (if (Variables|Default|GetLockActionEnabled)
      (Variables|Default|GetTargetLockActor ; Is the camera already locked on an actor?
        (:then
          (Variables|Default|SetTargetLockActor 0) ; Already has a targetlockactor. Set this to empty
          ;;[0.004712 0.07292 0] If the target is not locked, disable camera lock
          (Variables|/Script/Engine.CharacterMovementComponent|SetbOrientRotationToMovement _charactermovement_2 true)
          (Variables|/Script/Engine.CharacterMovementComponent|SetbUseControllerDesiredRotation _charactermovement_2 false)
          (Actor|DestroyActor (Variables|Default|GetTargetLockWidget)))
        (:else
          (bind (_outhit _returnvalue_3) (Collision|SphereTraceForObjects "0, 0, 0" (+ (Math|Vector|MakeVector (.x _returnvalue_2) (.y _returnvalue_2) (+ (.z _returnvalue_2) 2e+01)) (* (Math|Vector|GetForwardVector (Transformation|GetWorldRotation _transformcomponent)) 1e+03)) 1.5e+02 (Utilities|Array|MakeArray "ObjectTypeQuery3") false 0 "ForDuration" true "(R=1.000000,G=0.000000,B=0.000000,A=1.000000)" "(R=0.000000,G=1.000000,B=0.000000,A=1.000000)" 2.0))
          (if _returnvalue_3
            (Variables|Default|SetTargetLockActor (.HitActor (Collision|BreakHitResult _outhit)))
            ;;[0.004712 0.07292 0] If the target is locked, lock camera to face target
            (Variables|/Script/Engine.CharacterMovementComponent|SetbOrientRotationToMovement _charactermovement false)
            (Variables|/Script/Engine.CharacterMovementComponent|SetbUseControllerDesiredRotation _charactermovement true)
            (bind _returnvalue_4 (Game|SpawnActorfromClass "/Game/Blueprints/BP_TargetLockWidget.BP_TargetLockWidget_C" (Math|Transform|MakeTransform (Math|Vector|MakeVector (.x (.location (Transformation|GetActorTransform (Variables|Default|GetTargetLockActor)))) (.y (.location (Transformation|GetActorTransform (Variables|Default|GetTargetLockActor)))) (+ (.z (.location (Transformation|GetActorTransform (Variables|Default|GetTargetLockActor)))) 2e+01)) (.rotation (Transformation|GetActorTransform (Variables|Default|GetTargetLockActor))) "1.000000,1.000000,1.000000") "AlwaysSpawn" "MultiplyWithRoot" 0 0))
            (bind _output_get (Variables|Default|SetTargetLockWidget _returnvalue_4))
            (Transformation|AttachActorToActor _output_get (Variables|Default|GetTargetLockActor) "None" "SnapToTarget" "KeepRelative" "SnapToTarget" true) ; Attach the lock widget to the actor being locked upon - snapped to target
          ))))))

(event Input|EnhancedActionEvents|EnhancedInputActionIA_SwordAttack
  (params (ActionValue :type Boolean) (ElapsedSeconds :type Float%20%28double-precision%29) (TriggeredSeconds :type Float%20%28double-precision%29) (InputAction :type Input%20Action%20Object%20Reference :default "/Game/ThirdPerson/Input/Actions/IA_SwordAttack.IA_SwordAttack"))
  ;[0.004712 0.07292 0] Sword Combo
  (:Started
    (if (not (Variables|Default|GetIsAttacking))
      (Variables|Default|SetIsAttacking true)
      (Animation|Montage|PlayMontage (Variables|/Script/Engine.Character|GetMesh (Variables|Default|GetPlayerBP)) "/Game/Characters/Souls/Combat/SwordAttackCombo_Montage.SwordAttackCombo_Montage"
        (:OnCompleted
          (Variables|Default|SetIsAttacking false :!label _label)
          (Variables|Default|SetCombo? false))
        (:OnInterrupted
          (goto _label))
        (:OnNotifyBegin
          (if (and (Variables|Default|GetIsAttacking) (Variables|Default|GetCombo?))
            (Variables|Default|SetCombo? false)
            (else
              (Animation|Montage|MontageStop (Components|SkeletalMesh|GetAnimInstance (Variables|/Script/Engine.Character|GetMesh (Variables|Default|GetPlayerBP))) 0.2 "/Game/Characters/Souls/Combat/SwordAttackCombo_Montage.SwordAttackCombo_Montage")))))
      (else
        (Variables|Default|SetCombo? true)))))

(event Input|EnhancedActionEvents|EnhancedInputActionIA_Dodge
  (params (ActionValue :type Boolean) (ElapsedSeconds :type Float%20%28double-precision%29) (TriggeredSeconds :type Float%20%28double-precision%29) (InputAction :type Input%20Action%20Object%20Reference :default "/Game/ThirdPerson/Input/Actions/IA_Dodge.IA_Dodge"))
  (:Triggered
    (if (not (Variables|Default|GetIsDodging?))
      (Variables|Default|SetIsDodging? true)
      (Utilities|FlowControl|Sequence
        (:then_0
          (if (Variables|/Script/Engine.CharacterMovementComponent|GetbUseControllerDesiredRotation (Variables|/Script/Engine.Character|GetCharacterMovement (Variables|Default|GetPlayerBP)))
            (switch string (Utilities|String|ToString(Text) (Class|KismetInputLibrary|KeyGetDisplayName (Variables|/Game/ThirdPerson/Blueprints/BP_ThirdPersonCharacter.BP_ThirdPersonCharacter_C|GetDirection%20Key (Variables|Default|GetPlayerBP)) true))
              (:W
                (Variables|Default|SetMovementDirection "NewEnumerator0"))
              (:A
                (Variables|Default|SetMovementDirection "NewEnumerator2"))
              (:S
                (Variables|Default|SetMovementDirection "NewEnumerator1"))
              (:D
                (Variables|Default|SetMovementDirection "NewEnumerator3")))
            (else
              (Variables|Default|SetMovementDirection "NewEnumerator0") ; If not using a movement input, default to Forward dodge
            )))
        (:then_1
          (Animation|Montage|PlayMontage (Variables|/Script/Engine.Character|GetMesh (Variables|Default|GetPlayerBP)) (Utilities|Select :Index (Variables|Default|GetMovementDirection) :NewEnumerator0 "/Game/Characters/Souls/Combat/Dodge/Dodge_F_Montage.Dodge_F_Montage" :NewEnumerator1 "/Game/Characters/Souls/Combat/Dodge/Dodge_B_Montage.Dodge_B_Montage" :NewEnumerator2 "/Game/Characters/Souls/Combat/Dodge/Dodge_L_Montage.Dodge_L_Montage" :NewEnumerator3 "/Game/Characters/Souls/Combat/Dodge/Dodge_R_Montage.Dodge_R_Montage")
            (:OnCompleted
              _)
            (:OnInterrupted
              _))
          (Variables|Default|SetIsDodging? false)
          (Development|PrintString (Utilities|String|ToString(Float) (Variables|Default|GetSwordDamage))))))))

(event EventTick
  (params (DeltaSeconds :type Float%20%28single-precision%29))
  (bind _playerbp (Variables|Default|GetPlayerBP))
  (bind _targetlockactor (Variables|Default|GetTargetLockActor))
  (bind _returnvalue (Transformation|GetActorLocation _targetlockactor))
  (bind _returnvalue_2 (Transformation|GetActorLocation _playerbp))
  (bind _returnvalue_3 (Math|Rotator|FindLookatRotation _returnvalue_2 _returnvalue))
  ;[0 0.06426 0.07292] Target Lock
  ;;[0.004712 0.07292 0] Target Lock Update
  (Variables|Default|GetTargetLockActor
    (:then
      (Pawn|SetControlRotation (Pawn|GetController (Variables|Default|GetPlayerBP)) (Math|Rotator|MakeRotator (.roll _returnvalue_3) (+ (.pitch _returnvalue_3) -2e+01) (.yaw _returnvalue_3))))
    (:else)))

(event EventBeginPlay
  ;[0.004712 0.07292 0] Get Player Class
  (bind _asbp_third_person_character (Utilities|Casting|CastToBP_ThirdPersonCharacter (Components|GetOwner)))
  (Variables|Default|SetPlayerBP _asbp_third_person_character))