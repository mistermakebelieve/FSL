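; BP_Enemy is an AI enemy with stat-driven health and a montage-based sword attack.
; Incoming damage lowers a value in BPCStats, which is linked to the enemy's widget health bar.
; Between begin and end trace events, a looping timer sphere-traces hilt to tip for pawns, with hits throttled by a fixed delay the author flags as needing animation-based timing.
; Die disables movement and ragdolls the mesh.
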(event Custom|DamageTrace
  ;[0.004712 0.07292 0] Sword Traces
  (if (not (Variables|Default|GetIsDead?))
    (bind (_outhit _returnvalue) (Collision|SphereTraceForObjects (Transformation|GetWorldLocation (Variables|Default|GetStart%20Sword%20Trace%20Pos)) (Transformation|GetWorldLocation (Variables|Default|GetEnd%20Sword%20Trace%20Pos)) 25.0 (Utilities|Array|MakeArray "ObjectTypeQuery3") false 0 "ForOneFrame"))
    (if _returnvalue
      (Utilities|FlowControl|DoOnce false :!label _label
        (:Completed
          (Game|Damage|ApplyDamage (.HitActor (Collision|BreakHitResult _outhit)) (Variables|Default|GetSwordDamage) 0 0)
          ;[0.6198 0.01517 0] !!!!!This is bad. It should be based on animation!!!!!
          (Utilities|FlowControl|Delay 0.3)
          (goto _label Reset))))))

(event EventBeginPlay
  (bind _aswb_enemy_health (Utilities|Casting|CastToWB_EnemyHealth (UserInterface|GetWidget (Variables|Default|GetWidget))))
  (Variables|/Game/Blueprints/BPC_Stats.BPC_Stats_C|SetHealth%20Progress%20Bar (Variables|Default|GetBPC_Stats) (Variables|/Game/UI/WB_EnemyHealth.WB_EnemyHealth_C|GetHealthBar _aswb_enemy_health)))

(event Game|Damage|EventAnyDamage
  (params (Damage :type Float%20%28single-precision%29) (DamageType :type Damage%20Type%20Object%20Reference) (InstigatedBy :type Controller%20Object%20Reference) (DamageCauser :type Actor%20Object%20Reference))
  (Default|AlterStatValue (Variables|Default|GetBPC_Stats) "NewEnumerator0" (* Damage -1.0)))

(event EventDie
  (Pawn|Components|CharacterMovement|DisableMovement (Variables|Character|GetCharacterMovement))
  (Physics|SetSimulatePhysics (Variables|Character|GetMesh) true))

(event EventBeginSwordTrace
  ;[0.004712 0.07292 0] Sword Traces
  (bind _returnvalue (Utilities|Time|SetTimerbyEvent (delegate Custom|DamageTrace) 0.01 true)))

(event EventEndSwordTrace
  ;[0.004712 0.07292 0] Sword Traces
  (if (Utilities|Time|IsValidTimerHandle (stale EventBeginSwordTrace _returnvalue))
    (Utilities|Time|ClearandInvalidateTimerbyHandle (stale EventBeginSwordTrace _returnvalue))))

(fn ConstructionScript)

(fn SwordAttack
  (bind _returnvalue (Animation|PlayAnimMontage "/Game/Characters/Souls/Combat/SwordAttackCombo_Montage.SwordAttackCombo_Montage" 1.0 "None"))
  (return _returnvalue))